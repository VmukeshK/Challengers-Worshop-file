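; Melee enemy character that chases player 0 and reports its death to BP_character's kill count.
; A looping AIMoveTo drives pursuit, while Tick pauses movement and plays the Slice montage within attack range.
; DamagePlayer applies hit damage but is not called within this graph.
; AnyDamage lowers health and calls KillAi only at exactly zero, stopping movement and setting Dead, which Tick does not check.
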(event Game|Damage|EventAnyDamage
  (params (Damage :type Float%20%28single-precision%29) (DamageType :type Damage%20Type%20Object%20Reference) (InstigatedBy :type Controller%20Object%20Reference) (DamageCauser :type Actor%20Object%20Reference))
  (bind _output_get (Variables|Default|SetHealth_AI (- (Variables|Default|GetHealth_AI) Damage)))
  (if (== _output_get 0.0)
    (CallFunction|KillAi)))

(event EventBeginPlay
  (if (not (Variables|Default|GetDead)) :!label _label
    (AI|AIMoveTo self "0, 0, 0" (Game|GetPlayerCharacter 0) 1e+01 false
      (:OnSuccess
        _)
      (:OnFail
        _))
    (Utilities|FlowControl|Delay 0.2)
    (goto _label)))

(event EventTick
  (params (DeltaSeconds :type Float%20%28single-precision%29))
  (if (and (CallFunction|IsWithinAttackRange) (not (CallFunction|IsAttacking)))
    (Components|Activation|Deactivate (Variables|Character|GetCharacterMovement))
    (Animation|Montage|PlayMontage (Variables|Character|GetMesh) "/Game/Character/enemy/anim/slice_montage.slice_montage"
      (:OnCompleted
        (Components|Activation|Activate (Variables|Character|GetCharacterMovement) false)))))

(fn ConstructionScript)

(fn IsWithinAttackRange
  (return (< (Transformation|GetDistanceTo (Game|GetPlayerCharacter 0)) (Variables|Default|GetAtttack%20range))))

(fn IsAttacking
  (return (Animation|Montage|MontageIsPlaying (Components|SkeletalMesh|GetAnimInstance (Variables|Character|GetMesh)) "/Game/Character/enemy/anim/slice_montage.slice_montage")))

(fn DamagePlayer
  (Game|Damage|ApplyDamage (Game|GetPlayerCharacter 0) (Variables|Default|GetDamagePerHit) 0 0))

(fn KillAi
  (bind _charactermovement (Variables|Character|GetCharacterMovement))
  (Variables|Default|SetDead true)
  (Components|Movement|StopMovementImmediately _charactermovement)
  (Components|Activation|Deactivate _charactermovement)
  (bind _asbp_character (Utilities|Casting|CastToBP_character (Game|GetPlayerCharacter 0)))
  (Default|IncKill _asbp_character))